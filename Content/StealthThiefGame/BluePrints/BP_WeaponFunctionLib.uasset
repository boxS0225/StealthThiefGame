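; BP_WeaponFunctionLib is a function library that provides weapon parameter lookup and reload math.
; GetWeaponParamTable scans the rows of WeaponParamDataTable and returns the one whose WeaponTag matches the given weapon name.
; GetCapacity reads Capacity from that row, and ReLoadProcess uses it to move as much held ammo as fits into the remaining count.
; The reload only computes and returns the updated counts, amount added and weapon name.
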(fn `GetCapacity`
  (params (weaponName :type Name))
  (returns (Capacity :type Integer))
  (bind `_外側の列` (`self.GetWeaponParamTable` weaponName))
  (return (`.Capacity` (break `WeaponParamStruct` `_外側の列`))))

(fn `GetWeaponParamTable`
  (params (WeaponName :type Name))
  (returns (`外側の列` :type "WeaponParamStruct Structure"))
  (bind _outrownames (`DataTableFunctionLibrary.GetDataTableRowNames` "/Game/StealthThiefGame/Player/Weapons/WeaponParamDataTable.WeaponParamDataTable"))
  (for _array_element _outrownames
    (bind _returnvalue (`|GetDataTableRow` "/Game/StealthThiefGame/Player/Weapons/WeaponParamDataTable.WeaponParamDataTable" _array_element)
      (:`then`
        (if (== (`.WeaponTag` (break `WeaponParamStruct` _returnvalue)) WeaponName)
          (return _returnvalue))))))

(fn `ReLoadProcess`
  (params (WeaponName :type Name) (Remain :type Integer) (Hold :type Integer))
  (returns (UpdataRemain :type Integer) (UpdataHold :type Integer) (ReturnWeaponName :type Name) (Add :type Integer))
  (locals (AddAmmo :type Integer :default 0))
  (bind _capacity (`self.GetCapacity` WeaponName))
  (bind _returnvalue (`KismetMathLibrary.Min` (- _capacity Remain) Hold))
  (bind _output_get (set `local.AddAmmo` _returnvalue))
  (return (+ _returnvalue Remain) (- Hold _output_get) WeaponName _output_get))