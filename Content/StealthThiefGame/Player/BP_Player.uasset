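; Player character Blueprint for the stealth thief game, handling spawn, sprint, reload and death/respawn.
; Dissolve materials on body and logo meshes animate at spawn, then attach weapons to sockets, and again on death before destroying and respawning via BP_STGame.
; Reloads pass an ammo and state check, play a montage, then update ammo and HUD on ReloadNotify, with separate shotgun logic.
; Sprint eases walk speed through a reversible timeline; G applies debug self-damage.
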(event EventBeginPlay
  (bind _returnvalue (Class|StealthThiefGameCharacter|GetDissolveMesh))
  (bind _returnvalue_2 (Class|StealthThiefGameCharacter|GetDissolveMesh))
  (bind _mesh (Variables|Character|GetMesh))
  ;[1 1 1] スタート
  (|CallParentFunction)
  (bind _returnvalue_3 (Class|DissolveMesh|CreateDissolveMesh _returnvalue _mesh))
  (Class|StealthThiefGameCharacter|SetBodyMesh _returnvalue_3)
  (bind _returnvalue_4 (Class|DissolveMesh|CreateDissolveMesh _returnvalue _mesh 1))
  (Class|StealthThiefGameCharacter|SetLogoMesh _returnvalue_4)
  (bind _dissolve (Timeline|DissolveTimeLine Play)
    (:Update
      (Class|DissolveMesh|SetMaterialParameter _returnvalue_2 (Class|StealthThiefGameCharacter|GetBodyMesh) "Rate" _dissolve)
      (Class|DissolveMesh|SetMaterialParameter _returnvalue_2 (Class|StealthThiefGameCharacter|GetLogoMesh) "Rate" _dissolve))
    (:Finished
      (bind _outactors (Actor|GetAllActorsOfClass "/Script/StealthThiefGame.WeaponBase"))
      (for _array_element _outactors
        (Class|WeaponInterface|SetPlayerSocket _array_element)))))

(event EventReloadNotify
  (bind _returnvalue (Class|StealthThiefGameCharacter|GetWeaponName))
  (bind _returnvalue_2 (Class|StealthThiefGameCharacter|GetWeaponName))
  (bind _returnvalue_3 (Class|StealthThiefGameCharacter|GetWeaponName))
  (bind (__remainammo __holdammo) (Class|StealthThiefGameCharacter|GetNumberOfAmmo _returnvalue_2))
  (bind (__remainammo_2 __holdammo_2) (Class|StealthThiefGameCharacter|GetNumberOfAmmo _returnvalue))
  (bind (__remainammo_3 __holdammo_3) (Class|StealthThiefGameCharacter|GetNumberOfAmmo _returnvalue_3))
  (if (== "ShotGun" _returnvalue_2)
    (bind (_returnweaponname _updataremain _updatahold) (CallFunction|ReLoadShotGun _returnvalue_2 __remainammo __holdammo))
    (Class|StealthThiefGameCharacter|SetNuberOfAmmo _returnweaponname _updataremain _updatahold)
    (Class|WidgetInterface|SetAmmoWidget(Message) (Class|StealthThiefGameCharacter|GetAmmoWidget) __remainammo_2 __holdammo_2)
    (else
      (bind (_returnweaponname_2 _updataremain_2 _updatahold_2) (CallFunction|ReLoadProcess _returnvalue_2 __remainammo __holdammo))
      (Class|StealthThiefGameCharacter|SetNuberOfAmmo _returnweaponname_2 _updataremain_2 _updatahold_2)
      (Class|WidgetInterface|SetAmmoWidget(Message) (Class|StealthThiefGameCharacter|GetAmmoWidget) __remainammo_3 __holdammo_3))))

(event EventSprintReleased
  (params (_value :type Input%20Action%20Value%20Structure%20%28by%20ref%29))
  (bind _floatspeed (Timeline|Sprint_Timeline Reverse)
    (:Update
      (Variables|/Script/Engine.CharacterMovementComponent|SetMaxWalkSpeed (Variables|Character|GetCharacterMovement) _floatspeed))))

(event EventTick
  (params (DeltaSeconds :type Float%20%28single-precision%29)))

(event EventReLoad
  (params (_value :type Input%20Action%20Value%20Structure%20%28by%20ref%29))
  (bind _returnvalue (Class|StealthThiefGameCharacter|GetWeaponName))
  (bind (__remainammo __holdammo) (Class|StealthThiefGameCharacter|GetNumberOfAmmo _returnvalue))
  (Utilities|ReloadCheck
    (:true
      (Class|StealthThiefGameCharacter|SetIsReload true)
      (bind _add (CallFunction|ReLoadProcess _returnvalue __remainammo __holdammo))
      (bind _returnvalue_2 (Animation|PlayAnimMontage (Class|StealthThiefGameCharacter|GetReloadAnim) 1.0 "None"))
      (Class|AnimInterface|ReloadCount(Message) (Class|StealthThiefGameCharacter|GetMyAnimInstance) _add)
      (Utilities|FlowControl|Delay _returnvalue_2)
      (Class|StealthThiefGameCharacter|SetIsReload false))))

(event EventDestroyed
  (bind _asbp_stgame (Utilities|Casting|CastToBP_STGame (Game|GetGameMode)))
  (Default|CallOnPlayerDie _asbp_stgame self))

(event EventReStartPlayer
  (bind _returnvalue (Class|StealthThiefGameCharacter|GetDissolveMesh))
  ;[1 1 1] 死亡判定
  (bind _dissolve (Timeline|タイムライン Play)
    (:Update
      (Class|DissolveMesh|SetMaterialParameter _returnvalue (Class|StealthThiefGameCharacter|GetBodyMesh) "Rate" _dissolve)
      (Class|DissolveMesh|SetMaterialParameter _returnvalue (Class|StealthThiefGameCharacter|GetLogoMesh) "Rate" _dissolve))
    (:Finished
      (Widget|RemovefromParent (Class|StealthThiefGameCharacter|GetCurrentHpWidget))
      (CallFunction|ReStart))))

(event EventSprintPressed
  (params (_value :type Input%20Action%20Value%20Structure%20%28by%20ref%29))
  (bind _floatspeed (Timeline|Sprint_Timeline Play)
    (:Update
      (Variables|/Script/Engine.CharacterMovementComponent|SetMaxWalkSpeed (Variables|Character|GetCharacterMovement) _floatspeed))))

(event Input|KeyboardEvents|DebugKeyG
  (params (Key :type Key%20Structure :default "None") (ActionValue :type Input%20Action%20Value%20Structure))
  (:Pressed
    (Game|Damage|ApplyDamage (Components|GetOwner (Variables|Character|GetMesh)) 5.0 0 0)))

(fn ConstructionScript)

(fn ReStart
  (LocalVariables|SetController%20Ref (Pawn|GetController))
  (Actor|DestroyActor)
  (bind _asbp_stgame (Utilities|Casting|CastToBP_STGame (Game|GetGameMode)))
  (Class|GameModeBase|RestartPlayer _asbp_stgame (LocalVariables|GetController%20Ref)))