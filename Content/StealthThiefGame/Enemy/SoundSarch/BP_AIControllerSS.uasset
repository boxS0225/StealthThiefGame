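; AI controller for the SoundSarch enemy in the stealth thief game, starting the BT_SoundSarch behavior tree on BeginPlay.
; AI Perception updates feed the Blackboard, branching on the stimulus sense class.
; Sight sets TargetActor to the seen actor, or clears it when sight is lost.
; Any other sense writes isHeard from the sensed result and stores the stimulus location in TargetLocation.
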(event `self.ReceiveBeginPlay`
  (`self.RunBehaviorTree` "/Game/StealthThiefGame/Enemy/SoundSarch/BT_SoundSarch.BT_SoundSarch"))

(event `self.AIPerception.OnTargetPerceptionUpdated`
  (params (Actor :type "Actor Object Reference") (Stimulus :type "AIStimulus Structure"))
  (bind (_age _expirationage _strength _stimuluslocation _receiverlocation _tag _bsuccessfullysensed) (break `AIStimulus` Stimulus))
  (bind _returnvalue (`AIBlueprintHelperLibrary.GetBlackboard` null))
  (bind _returnvalue_2 (`AIBlueprintHelperLibrary.GetBlackboard` null))
  (bind _returnvalue_3 (`AIPerceptionSystem.GetSenseClassForStimulus` Stimulus))
  (if (== _returnvalue_3 "/Script/AIModule.AISense_Sight")
    (if _bsuccessfullysensed
      (`BlackboardComponent.SetValueAsObject` _returnvalue_2 "TargetActor" Actor)
      (else
        (`BlackboardComponent.SetValueAsObject` _returnvalue_2 "TargetActor" null)))
    (else
      (`BlackboardComponent.SetValueAsBool` _returnvalue "isHeard" _bsuccessfullysensed)
      (`BlackboardComponent.SetValueAsVector` _returnvalue "TargetLocation" _stimuluslocation))))

(fn `UserConstructionScript`)